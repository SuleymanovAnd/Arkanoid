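; BP_CubeDestructable is a grid of destructible cubes for a ball-and-rocket brick breaker.
; The construction script builds an X-by-Y loop of static mesh components, tracking each one's life in a map.
; Ball or rocket hits reduce that life; depleted cubes are destroyed, with a random chance to spawn one of two bonuses.
; LiveCubes decrements only on that bonus branch, and reaching zero calls AllCubesDead.
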(event Custom|Bonus
  (params (Component :type Primitive%20Component%20Object%20Reference))
  (bind _returnvalue (Transformation|GetWorldLocation Component))
  (bind _returnvalue_2 (Math|Conversions|ToTransform(Vector) _returnvalue))
  (if (Math|Random|RandomBoolwithWeight 0.5)
    (Game|SpawnActorfromClass "/Game/Blueprints/Construction/BP_Bonus_Size.BP_Bonus_Size_C" _returnvalue_2 "AlwaysSpawn" 0 0)
    (else
      (Game|SpawnActorfromClass "/Game/Blueprints/Construction/BP_Bonus.BP_Bonus_C" _returnvalue_2 "AlwaysSpawn" 0 0))))

(event EventBeginPlay)

(event EventTick
  (params (DeltaSeconds :type Float%20%28single-precision%29)))

(event Collision|EventHit
  (params (MyComp :type Primitive%20Component%20Object%20Reference) (Other :type Actor%20Object%20Reference) (OtherComp :type Primitive%20Component%20Object%20Reference) (bSelfMoved :type Boolean) (HitLocation :type Vector :default "0, 0, 0") (HitNormal :type Vector :default "0, 0, 0") (NormalImpulse :type Vector :default "0, 0, 0") (Hit :type Hit%20Result%20Structure%20%28by%20ref%29))
  (bind _grouplife (Variables|Default|GetGroupLife))
  (Utilities|Casting|CastToBP_Ball Other
    (:then
      _)
    (:CastFailed
      (Utilities|Casting|CastToBP_Rocket Other)))
  (bind _result (Math|Integer|DecrementInt (.Value (Utilities|Map|Find _grouplife MyComp)))
    (:%20%20
      (Utilities|Map|Add _grouplife MyComp _result)
      (if (<= _result 0)
        (if (Math|Random|RandomBoolwithWeight 0.5)
          (CallFunction|Bonus MyComp)
          (Math|Integer|DecrementInt (Variables|Default|GetLiveCubes)
            (:%20%20
              _)))
        (Components|DestroyComponent MyComp)
        (if (<= (Variables|Default|GetLiveCubes) 0)
          (Default|CallAllCubesDead))))))

(fn ConstructionScript
  (for _index (range 0 (Variables|Default|GetX))
    (for _index_2 (range 0 (Variables|Default|GetY))
      (bind _returnvalue (AddComponent|AddStaticMeshComponent false (Math|Transform|MakeTransform (Math|Vector|MakeVector (Math|Conversions|ToFloat(Integer) (* _index (Variables|Default|GetPadding))) (Math|Conversions|ToFloat(Integer) (* _index_2 (Variables|Default|GetPadding))) 0.0))))
      (Rendering|Material|SetMaterial _returnvalue 0 (Variables|Default|GetMaterial))
      (Utilities|Map|Add (Variables|Default|GetGroupLife) _returnvalue (Variables|Default|Getlife))
      (Math|Integer|IncrementInt (Variables|Default|GetLiveCubes)))))