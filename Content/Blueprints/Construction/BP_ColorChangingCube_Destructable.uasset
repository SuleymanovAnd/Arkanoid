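; Destructible cube Blueprint that recolors its components when hit and can spawn bonus pickups.
; On Hit, it sets the hit component's material by looking up its GroupLife value in the Materials map, then runs the parent hit logic.
; The Bonus event spawns a pickup at the component's location: a rocket bonus 18% of the time, otherwise a random size, standard or life bonus.
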(event EventBeginPlay
  (|CallParentFunction) ; This node is disabled and will not be called.\nDrag off pins to build functionality.
)

(event EventBonus
  (params (Component :type Primitive%20Component%20Object%20Reference))
  (bind _returnvalue (Transformation|GetWorldLocation Component))
  (bind _returnvalue_2 (Math|Conversions|ToTransform(Vector) _returnvalue))
  (switch int (Math|Integer|SelectInt 3 (Math|Random|RandomIntegerinRange 0 2) (Math|Random|RandomBoolwithWeight 0.18))
    (:0
      (Game|SpawnActorfromClass "/Game/Blueprints/Construction/BP_Bonus_Size.BP_Bonus_Size_C" _returnvalue_2 "AlwaysSpawn" 0 0))
    (:1
      (Game|SpawnActorfromClass "/Game/Blueprints/Construction/BP_Bonus.BP_Bonus_C" _returnvalue_2 "AlwaysSpawn" 0 0))
    (:2
      (Game|SpawnActorfromClass "/Game/Blueprints/Construction/BP_BonusLive.BP_BonusLive_C" _returnvalue_2 "AlwaysSpawn" 0 0))
    (:3
      (Game|SpawnActorfromClass "/Game/Blueprints/Construction/BP_BonusRocket.BP_BonusRocket_C" _returnvalue_2 "AlwaysSpawn" 0 0))))

(event EventTick
  (params (DeltaSeconds :type Float%20%28single-precision%29))
  (|CallParentFunction DeltaSeconds) ; This node is disabled and will not be called.\nDrag off pins to build functionality.
)

(event Collision|EventHit
  (params (MyComp :type Primitive%20Component%20Object%20Reference) (Other :type Actor%20Object%20Reference) (OtherComp :type Primitive%20Component%20Object%20Reference) (bSelfMoved :type Boolean) (HitLocation :type Vector :default "0, 0, 0") (HitNormal :type Vector :default "0, 0, 0") (NormalImpulse :type Vector :default "0, 0, 0") (Hit :type Hit%20Result%20Structure%20%28by%20ref%29))
  (CallFunction|ColorChange MyComp MyComp)
  (|CallParentFunction MyComp Other OtherComp bSelfMoved HitLocation HitNormal NormalImpulse Hit))

(fn ConstructionScript
  (|CallParentFunction))

(fn ColorChange
  (params (Target :type Primitive%20Component%20Object%20Reference) (Component :type Actor%20Component%20Object%20Reference%20%28by%20ref%29))
  (Rendering|Material|SetMaterial Target 0 (.Value (Utilities|Map|Find (Variables|Default|GetMaterials) (.Value (Utilities|Map|Find (Variables|Default|GetGroupLife) Component))))))