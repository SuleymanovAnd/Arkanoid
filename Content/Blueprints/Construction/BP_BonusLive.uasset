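; BP_BonusLive is a bonus actor that randomly becomes either a plus-life or minus-life pickup.
; On BeginPlay a weighted 50% roll can swap the mesh to SM_Minus and apply the minus material to the mesh and BonusBalls.
; OnBonus reuses the SetStaticMesh return value as the variant flag, calls CallMinusLive or CallPlusLive accordingly, then destroys the actor.
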(event EventBeginPlay
  (bind _staticmesh (Variables|Default|GetStaticMesh))
  (if (Math|Random|RandomBoolwithWeight 0.5)
    _
    (else
      (bind _returnvalue (Components|StaticMesh|SetStaticMesh _staticmesh "/Game/Meshes/SM_Minus.SM_Minus"))
      (for _index (range 0 2)
        (Rendering|Material|SetMaterial _staticmesh _index "/Game/Environment/Materials/MI_BonusMinusLive.MI_BonusMinusLive"))
      (for _index_2 (range 0 2)
        (Rendering|Material|SetMaterial (Variables|Default|GetBonusBalls) _index_2 "/Game/Environment/Materials/MI_BonusMinusLive.MI_BonusMinusLive"))))
  (|CallParentFunction))

(event Collision|EventActorBeginOverlap
  (params (OtherActor :type Actor%20Object%20Reference))
  (|CallParentFunction OtherActor) ; This node is disabled and will not be called.\nDrag off pins to build functionality.
)

(event EventTick
  (params (DeltaSeconds :type Float%20%28single-precision%29))
  (|CallParentFunction DeltaSeconds))

(event EventOnBonus
  (params (Object :type BP%20Pawn%20Object%20Reference))
  (if (stale EventBeginPlay _returnvalue)
    (Default|CallMinusLive)
    (Actor|DestroyActor)
    (else
      (Default|CallPlusLive)
      (Actor|DestroyActor))))

(fn ConstructionScript
  (|CallParentFunction))