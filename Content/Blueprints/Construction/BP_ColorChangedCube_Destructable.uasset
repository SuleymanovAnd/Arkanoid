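; Destructible cube Blueprint that changes a struck component's material according to its remaining life.
; On Hit, it looks up the component's value in the GroupLife map and uses it as the key into the Materials map for the new material.
; It prints the life value for debugging, then calls the parent Hit, so the material reflects life before any parent handling runs.
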(event EventBeginPlay
  (|CallParentFunction) ; This node is disabled and will not be called.\nDrag off pins to build functionality.
)

(event EventTick
  (params (DeltaSeconds :type Float%20%28single-precision%29))
  (|CallParentFunction DeltaSeconds) ; This node is disabled and will not be called.\nDrag off pins to build functionality.
)

(event Collision|EventHit
  (params (MyComp :type Primitive%20Component%20Object%20Reference) (Other :type Actor%20Object%20Reference) (OtherComp :type Primitive%20Component%20Object%20Reference) (bSelfMoved :type Boolean) (HitLocation :type Vector :default "0, 0, 0") (HitNormal :type Vector :default "0, 0, 0") (NormalImpulse :type Vector :default "0, 0, 0") (Hit :type Hit%20Result%20Structure%20%28by%20ref%29))
  (bind _grouplife (Variables|Default|GetGroupLife))
  (bind _value (Utilities|Map|Find _grouplife MyComp))
  (Development|PrintString (Utilities|String|ToString(Integer) _value))
  (Development|PrintString "life")
  (Rendering|Material|SetMaterial MyComp 0 (.Value (Utilities|Map|Find (Variables|Default|GetMaterials) _value)))
  (|CallParentFunction MyComp Other OtherComp bSelfMoved HitLocation HitNormal NormalImpulse Hit))

(fn ConstructionScript
  (|CallParentFunction))