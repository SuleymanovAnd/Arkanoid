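; Player controller that drives the player's BP_Pawn, shows the HUD and handles the end of the game.
; It caches the possessed pawn and moves it along world X from the Move Right axis, using its Speed, frame delta and a swept offset.
; FinishGame is bound to destructible-cube all-dead and pawn game-over events.
; After a delay, it swaps the info widget for the finish menu with UI-only input and cursor.
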(event Custom|FinishGame
  (bind _self self)
  (Utilities|FlowControl|Delay 3.0)
  (Widget|SetVisibility (Variables|Default|GetInfo) "Hidden")
  (bind _returnvalue (UserInterface|CreateWidget "/Game/UI/WBP_FinishMenu.WBP_FinishMenu_C" _self))
  (UserInterface|Viewport|AddtoViewport _returnvalue 0)
  (Input|SetInputModeUIOnly _self _returnvalue "LockOnCapture")
  (Variables|Default|SetbShowMouseCursor true))

(event EventPossess
  (params (PossessedPawn :type Pawn%20Object%20Reference))
  (bind _asbp_pawn (Utilities|Casting|CastToBP_Pawn PossessedPawn))
  (Variables|Default|SetBP%20MyPawn _asbp_pawn))

(event EventBeginPlay
  (bind _self self)
  (Utilities|FlowControl|Sequence
    (:then_0
      (Input|SetInputModeGameOnly _self)
      (bind _returnvalue (UserInterface|CreateWidget "/Game/UI/WBP_Info.WBP_Info_C" _self))
      (UserInterface|Viewport|AddtoViewport _returnvalue 0)
      (Variables|Default|SetInfo _returnvalue))
    (:then_1
      (bind _outactors (Actor|GetAllActorsOfClass "/Game/Blueprints/Construction/BP_CubeDestructable.BP_CubeDestructable_C"))
      (EventDispatchers|BindEventtoAllCubesDead _outactors (delegate Custom|FinishGame)))
    (:then_2
      (bind _outactors_2 (Actor|GetAllActorsOfClass "/Game/Blueprints/Construction/BP_Pawn.BP_Pawn_C"))
      (EventDispatchers|BindEventtoGameOver _outactors_2 (delegate Custom|FinishGame)))))

(event Input|AxisEvents|InputAxisMoveRight
  (params (AxisValue :type Float%20%28single-precision%29))
  (Transformation|AddActorWorldOffset (Variables|Default|GetBP%20MyPawn) (Math|Vector|MakeVector (* AxisValue (Variables|/Game/Blueprints/Construction/BP_Pawn.BP_Pawn_C|GetSpeed (Variables|Default|GetBP%20MyPawn)) (Utilities|Time|GetWorldDeltaSeconds)) 0.0 0.0) true))

(fn ConstructionScript)